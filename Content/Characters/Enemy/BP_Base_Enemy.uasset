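; Base enemy character Blueprint that plays an optional dissolve entry effect when it begins play.
; When UseEntryFX is set, it initializes the dissolve amount, then runs the EntryFX timeline with its play rate scaled by EntryFXTime.
; DissolveUpdate pushes each timeline value to the DissolveAmount material parameter on every skeletal mesh component and on the left and right weapon meshes from EnemyCombatComponent's equipped weapon.
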(event `self.ReceiveBeginPlay`
  (if (`self.bUseEntryFX`)
    (`self.DissolveUpdate` 1.0)
    (`TimelineComponent.SetPlayRate` (`self.EntryFX`) (/ 1.0 (`self.EntryFXTime`)))
    (bind (_direction _newtrack_0) (`Timeline|EntryFX`)
      (:`Update`
        (`self.DissolveUpdate` _newtrack_0)))))

(fn `DissolveUpdate`
  (params (ParameterValue :type "Float (double-precision)" :default 1.0))
  (bind _returnvalue (`PA_PawnCombatComponent.GetCharacterCurrentEquippingWeapon` (`self.EnemyCombatComponent`)))
  (bind _rightweaponmesh (`PA_BaseWeapon.RightWeaponMesh` _returnvalue))
  (for _array_element (`self.K2_GetComponentsByClass` self "/Script/Engine.SkeletalMeshComponent")
    (`MeshComponent.SetScalarParameterValueOnMaterials` _array_element "DissolveAmount" (`local.ParameterValue`))
    (`/Engine/EditorBlueprintResources/StandardMacros.IsValid` (`PA_PawnCombatComponent.GetCharacterCurrentEquippingWeapon` (`self.EnemyCombatComponent`))
      (:`Is Valid`
        (`|ExecutionSequence`
          (:`then_0`
            (`/Engine/EditorBlueprintResources/StandardMacros.IsValid` (`PA_BaseWeapon.LeftWeaponMesh` _returnvalue)
              (:`Is Valid`
                _)))
          (:`then_1`
            (`/Engine/EditorBlueprintResources/StandardMacros.IsValid` _rightweaponmesh
              (:`Is Valid`
                _))))
        (`MeshComponent.SetScalarParameterValueOnMaterials` _rightweaponmesh "DissolveAmount" (`local.ParameterValue`))
        (`MeshComponent.SetScalarParameterValueOnMaterials` (`PA_BaseWeapon.LeftWeaponMesh` _returnvalue) "DissolveAmount" (`local.ParameterValue`))))))

(fn `UserConstructionScript`)