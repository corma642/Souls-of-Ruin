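; BP_Goblin_Wizard is the wizard variant of the goblin enemy character, assembled from modular skeletal mesh pieces.
; Its construction script makes Mesh the leader pose component for the pants, hat, cloak, bracers, scroll and bottle, so they follow the body's animation, then runs the parent construction script.
; BeginPlay only calls the parent, so the Blueprint adds no gameplay logic in its graphs.
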(event `self.ReceiveBeginPlay`
  (`parent.ReceiveBeginPlay`))

(fn `UserConstructionScript`
  (`SkinnedMeshComponent.SetLeaderPoseComponent` (`self.SK_Wizard_Pants`) (`self.Mesh`) false false)
  (`SkinnedMeshComponent.SetLeaderPoseComponent` (`self.SK_Wizard_Hat`) (`self.Mesh`) false false)
  (`SkinnedMeshComponent.SetLeaderPoseComponent` (`self.SK_Wizard_Cloak`) (`self.Mesh`) false false)
  (`SkinnedMeshComponent.SetLeaderPoseComponent` (`self.SK_Wizard_Bracers`) (`self.Mesh`) false false)
  (`SkinnedMeshComponent.SetLeaderPoseComponent` (`self.SK_Wizard_Scroll`) (`self.Mesh`) false false)
  (`SkinnedMeshComponent.SetLeaderPoseComponent` (`self.SK_Wizard_Bottle`) (`self.Mesh`) false false)
  (`parent.UserConstructionScript`))