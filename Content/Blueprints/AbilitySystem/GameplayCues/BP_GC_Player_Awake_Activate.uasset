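; Gameplay cue notify for the player's Awake activation, showing rage visuals and audio while the cue is active.
; WhileActive plays a one-shot burst and sound at the target, then attaches a fire effect to the target's attach component.
; It also attaches effects to both meshes of the equipped weapon found through the pawn combat component.
; OnRemove destroys the three stored attached effects.
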(fn `OnRemove`
  (params (MyTarget :type "Actor Object Reference") (Parameters :type "GameplayCueParameters Structure (by ref)"))
  (returns (ReturnValue :type Boolean))
  (`|ExecutionSequence`
    (:`then_0`
      (bind _attachedragefx (`self.AttachedRageFX`)
        (:`then`
          (`ActorComponent.K2_DestroyComponent` _attachedragefx null))
        (:`else`)))
    (:`then_1`
      (bind _attachedleftweaponfx (`self.AttachedLeftWeaponFX`)
        (:`then`
          (`ActorComponent.K2_DestroyComponent` _attachedleftweaponfx null))
        (:`else`)))
    (:`then_2`
      (bind _attachedrightweaponfx (`self.AttachedRightWeaponFX`)
        (:`then`
          (`ActorComponent.K2_DestroyComponent` _attachedrightweaponfx null))
        (:`else`)))
    (:`then_3`
      (return false))))

(fn `UserConstructionScript`)

(fn `WhileActive`
  (params (MyTarget :type "Actor Object Reference") (Parameters :type "GameplayCueParameters Structure (by ref)"))
  (returns (ReturnValue :type Boolean))
  (locals (Weapon :type "PA_BaseWeapon Object Reference"))
  (`|ExecutionSequence`
    (:`then_0`
      (`NiagaraFunctionLibrary.SpawnSystemAtLocation` null "/Game/Assets/Niagara/Rage/NS_RageActivate.NS_RageActivate" (`self.K2_GetActorLocation` (`local.MyTarget`))))
    (:`then_1`
      (bind _returnvalue (`NiagaraFunctionLibrary.SpawnSystemAttached` "/Game/Assets/Niagara/Rage/NS_SampleSKFire.NS_SampleSKFire" (`.TargetAttachComponent` (`AbilitySystemBlueprintLibrary.BreakGameplayCueParameters` (`local.Parameters`))) "None" (0.0 0.0 0.0) (struct) "KeepRelativeOffset"))
      (set `self.AttachedRageFX` _returnvalue))
    (:`then_2`
      (`GameplayStatics.PlaySoundAtLocation` null "/Game/Blueprints/Sounds/Player/Awake/SW_Ability_FireBallCast01.SW_Ability_FireBallCast01" (`self.K2_GetActorLocation` (`local.MyTarget`)) (struct) 1.0 1.0 0.0 null null null null))
    (:`then_3`
      (bind _returnvalue_2 (`PA_FunctionLibrary.BP_GetPawnCombatComponentFromActor` (`local.MyTarget`))
        (:`Valid`
          (set `local.Weapon` (`PA_PawnCombatComponent.GetCharacterCurrentEquippingWeapon` _returnvalue_2))
          (`|ExecutionSequence`
            (:`then_0`
              (bind _returnvalue_3 (`NiagaraFunctionLibrary.SpawnSystemAttached` "/Game/Assets/MeleeWeaponAura_VFX/VFX/V4/NS_StylizedWeapon_V4_03.NS_StylizedWeapon_V4_03" (`PA_BaseWeapon.LeftWeaponMesh` (`local.Weapon`)) "None" (0.0 0.0 0.0) (struct) "KeepRelativeOffset"))
              (set `self.AttachedLeftWeaponFX` _returnvalue_3))
            (:`then_1`
              (bind _returnvalue_4 (`NiagaraFunctionLibrary.SpawnSystemAttached` "/Game/Assets/MeleeWeaponAura_VFX/VFX/V4/NS_StylizedWeapon_V4_03.NS_StylizedWeapon_V4_03" (`PA_BaseWeapon.RightWeaponMesh` (`local.Weapon`)) "None" (0.0 0.0 0.0) (struct) "KeepRelativeOffset"))
              (set `self.AttachedRightWeaponFX` _returnvalue_4))
            (:`then_2`
              (return false))))
        (:`InValid`
          (return false))))))