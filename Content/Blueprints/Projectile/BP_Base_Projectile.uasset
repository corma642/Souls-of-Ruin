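; Base projectile Blueprint that handles muzzle and impact visual effects, supporting both Cascade and Niagara assets.
; BeginPlay spawns whichever muzzle effects are set at the actor's location and forward rotation, tinting only the Cascade one.
; OnSpawnProjectileHitFX spawns impact effects at the hit location without auto-destroy, doubled in size when IsPlayer is false.
; Niagara impacts take their scale from MuzzleScale, while Cascade impacts use ImpactScale.
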(event `self.ReceiveBeginPlay`
  (`|ExecutionSequence`
    (:`then_0`
      (`/Engine/EditorBlueprintResources/StandardMacros.IsValid` (`self.Muzzle_Cascade`)
        (:`Is Valid`
          (`self.SpawnMuzzleCascadeEmitter`))))
    (:`then_1`
      (`/Engine/EditorBlueprintResources/StandardMacros.IsValid` (`self.Muzzle_Niagara`)
        (:`Is Valid`
          (`self.SpawnMuzzleNiagaraSystem`))))))

(event `self.BP_OnSpawnProjectileHitFX`
  (params (HitLocation :type "Vector Structure (by ref)") (IsPlayer :type Boolean))
  (`|ExecutionSequence`
    (:`then_0`
      (`/Engine/EditorBlueprintResources/StandardMacros.IsValid` (`self.Impact_Cascade`)
        (:`Is Valid`
          (`self.SpawnImpactCascadeEmitter` HitLocation IsPlayer))))
    (:`then_1`
      (`/Engine/EditorBlueprintResources/StandardMacros.IsValid` (`self.Impact_Niagara`)
        (:`Is Valid`
          (`self.SpawnImpactNiagaraSystem` HitLocation IsPlayer))))))

(fn `SpawnImpactCascadeEmitter`
  (params (HitLocation :type "Vector Structure") (IsPlayer :type Boolean))
  (if IsPlayer
    (`GameplayStatics.SpawnEmitterAtLocation` (`self.Impact_Cascade`) (`local.HitLocation`) (struct) (`KismetMathLibrary.Conv_DoubleToVector` (`self.Impact_Scale`)) false)
    (else
      (`GameplayStatics.SpawnEmitterAtLocation` (`self.Impact_Cascade`) (`local.HitLocation`) (struct) (* (`KismetMathLibrary.Conv_DoubleToVector` (`self.Impact_Scale`)) 2.0) false))))

(fn `SpawnImpactNiagaraSystem`
  (params (HitLocation :type "Vector Structure") (IsPlayer :type Boolean))
  (if IsPlayer
    (`NiagaraFunctionLibrary.SpawnSystemAtLocation` (`self.Impact_Niagara`) (`local.HitLocation`) (struct) (`KismetMathLibrary.Conv_DoubleToVector` (`self.Muzzle_Scale`)) false)
    (else
      (`NiagaraFunctionLibrary.SpawnSystemAtLocation` (`self.Impact_Niagara`) (`local.HitLocation`) (struct) (* (`KismetMathLibrary.Conv_DoubleToVector` (`self.Muzzle_Scale`)) 2.0) false))))

(fn `SpawnMuzzleCascadeEmitter`
  (bind _returnvalue (`GameplayStatics.SpawnEmitterAtLocation` (`self.Muzzle_Cascade`) (`self.K2_GetActorLocation`) (`KismetMathLibrary.Conv_VectorToRotator` (`self.GetActorForwardVector`)) (`KismetMathLibrary.Conv_DoubleToVector` (`self.Muzzle_Scale`))))
  (`FXSystemComponent.SetVectorParameter` _returnvalue "color" (`KismetMathLibrary.Conv_LinearColorToVector` (`self.Muzzle_Color`))))

(fn `SpawnMuzzleNiagaraSystem`
  (`NiagaraFunctionLibrary.SpawnSystemAtLocation` (`self.Muzzle_Niagara`) (`self.K2_GetActorLocation`) (`KismetMathLibrary.Conv_VectorToRotator` (`self.GetActorForwardVector`)) (`KismetMathLibrary.Conv_DoubleToVector` (`self.Muzzle_Scale`))))

(fn `UserConstructionScript`)